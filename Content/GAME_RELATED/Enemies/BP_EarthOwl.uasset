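; BP_EarthOwl is an earth owl enemy character with health, a melee attack, dash reaction and stun.
; Attack damages the player overlapping its sphere, then signals attack end after a delay; the montage step is an unwired placeholder.
; A dash hit costs health, then briefly grants invulnerability and ignores Pawn collision.
; Stun launches it away from the player and switches AIC_Enemy_Earth to stunned, then back to attacking.
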(event `self.ReceiveBeginPlay`
  (set `self.EnemyHealth` (`self.MAXEnemyHealth`)))

(event `GetDamaged`
  (if (>= (`self.EnemyHealth`) 1)
    (if (`self.CanGetDamaged`)
      (set `self.EnemyHealth` (- (`self.EnemyHealth`) 1))
      (`KismetSystemLibrary.PrintString` "ENEMY -1 HP"))
    (else
      (`KismetSystemLibrary.PrintString` " ENEMY DEAD")
      (`self.K2_DestroyActor`))))

(event `Attack`
  (set `self.IsAtt?` true)
  (if (`KismetArrayLibrary.Array_IsNotEmpty` (`PrimitiveComponent.GetOverlappingActors` (`self.Sphere`) "/Game/ThirdPerson/Blueprints/BP_ThirdPersonCharacter.BP_ThirdPersonCharacter_C"))
    (bind _asbp_third_person_character (cast `/Game/ThirdPerson/Blueprints/BP_ThirdPersonCharacter` (`GameplayStatics.GetPlayerCharacter` 0)))
    (`/Game/ThirdPerson/Blueprints/BP_ThirdPersonCharacter.GetDamaged` _asbp_third_person_character)
    (`KismetSystemLibrary.Delay` 3.0)
    (`self.OnAttackEnd`)
    (set `self.IsAtt?` false)))

(event `/Game/GAME_RELATED/InteractableObjects/PickingObjectsCode/BPI_DashBehavior.DashReaction`
  (`self.GetDamaged`)
  (set `self.CanGetDamaged` false)
  (`PrimitiveComponent.SetCollisionResponseToChannel` (`self.CapsuleComponent`) "ECC_Pawn" "ECR_Ignore")
  (`PrimitiveComponent.SetCollisionResponseToChannel` (`self.Mesh`) "ECC_Pawn" "ECR_Ignore")
  (`KismetSystemLibrary.Delay` 0.2)
  (set `self.CanGetDamaged` true)
  (`PrimitiveComponent.SetCollisionResponseToChannel` (`self.CapsuleComponent`) "ECC_Pawn" "ECR_Block")
  (`PrimitiveComponent.SetCollisionResponseToChannel` (`self.Mesh`) "ECC_Pawn" "ECR_Block"))

(event `GetStunned`
  (`self.LaunchCharacter` (* (`KismetMathLibrary.GetDirectionUnitVector` (`SceneComponent.K2_GetComponentLocation` (`Actor.RootComponent` (`GameplayStatics.GetPlayerCharacter` 0))) (`SceneComponent.K2_GetComponentLocation` (`self.RootComponent`))) (`self.Force`)) true)
  (bind _asaic_enemy_earth (cast `/Game/GAME_RELATED/Enemies/AI/AIC_Enemy_Earth` (`AIBlueprintHelperLibrary.GetAIController` self)))
  (`/Game/GAME_RELATED/Enemies/AI/AIC_Enemy_Earth.SetStateAsStunned` _asaic_enemy_earth)
  (`KismetSystemLibrary.Delay` 3.0)
  (bind _asaic_enemy_earth_2 (cast `/Game/GAME_RELATED/Enemies/AI/AIC_Enemy_Earth` (`AIBlueprintHelperLibrary.GetAIController` self)))
  (`/Game/GAME_RELATED/Enemies/AI/AIC_Enemy_Earth.SetStateAsAttacking` _asaic_enemy_earth_2))

(fn `UserConstructionScript`)