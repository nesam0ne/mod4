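; BP_Button is a puzzle button that activates a linked ControlledActor and plays a push sound.
; An overlapping BP_PickableCube triggers it, requiring a matching color when ColorPuzzle is set, and sends OnActivateMessage with the button's color.
; DashReaction also triggers it, but only once and with an empty color.
; End overlap does nothing, as the deactivation logic is disconnected, so the button never sends a deactivate message.
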(event `self.CubeCheck.OnComponentBeginOverlap`
  (params (OverlappedComponent :type "PrimitiveComponent Object Reference") (OtherActor :type "Actor Object Reference") (OtherComp :type "PrimitiveComponent Object Reference") (OtherBodyIndex :type Integer) (bFromSweep :type Boolean) (SweepResult :type "HitResult Structure (by ref)"))
  (if (== (`GameplayStatics.GetObjectClass` OtherActor) "/Game/GAME_RELATED/InteractableObjects/BP_PickableCube.BP_PickableCube_C")
    (if (`self.ColorPuzzle`)
      (bind _asbp_pickable_cube (cast `/Game/GAME_RELATED/InteractableObjects/BP_PickableCube` OtherActor))
      (if (`KismetStringLibrary.EqualEqual_StrStr` (`/Game/GAME_RELATED/InteractableObjects/BP_PickableCube.Color` _asbp_pickable_cube) (`self.ButtonColor`))
        (`GameplayStatics.PlaySound2D` "/Game/GAME_RELATED/Sounds/ButtonPush.ButtonPush" 1.0 1.0 0.0 null null :!label _label)
        (message `/Game/GAME_RELATED/InteractableObjects/BPI_ButtonAction.OnActivate` (`self.ControlledActor`) self (`self.ButtonColor`)))
      (else
        (goto _label)))))

(event `self.CubeCheck.OnComponentEndOverlap`
  (params (OverlappedComponent :type "PrimitiveComponent Object Reference") (OtherActor :type "Actor Object Reference") (OtherComp :type "PrimitiveComponent Object Reference") (OtherBodyIndex :type Integer)))

(event `/Game/GAME_RELATED/InteractableObjects/PickingObjectsCode/BPI_DashBehavior.DashReaction`
  (`/Engine/EditorBlueprintResources/StandardMacros.DoOnce` false
    (:`Completed`
      (`GameplayStatics.PlaySound2D` "/Game/GAME_RELATED/Sounds/ButtonPush.ButtonPush" 1.0 1.0 0.0 null null)
      (message `/Game/GAME_RELATED/InteractableObjects/BPI_ButtonAction.OnActivate` (`self.ControlledActor`) self ""))))

(fn `UserConstructionScript`)