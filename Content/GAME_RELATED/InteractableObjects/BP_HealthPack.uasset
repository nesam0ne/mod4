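; BP_HealthPack is a pickup that restores one point of health to the player character when touched.
; A sphere overlap casts to BP_ThirdPersonCharacter and only acts if current health is below maximum, then increments it and refreshes the UI.
; After a short delay the pack destroys itself and plays a 2D recharge sound.
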(event `self.Sphere.OnComponentBeginOverlap`
  (params (OverlappedComponent :type "PrimitiveComponent Object Reference") (OtherActor :type "Actor Object Reference") (OtherComp :type "PrimitiveComponent Object Reference") (OtherBodyIndex :type Integer) (bFromSweep :type Boolean) (SweepResult :type "HitResult Structure (by ref)"))
  (bind _asbp_third_person_character (cast `/Game/ThirdPerson/Blueprints/BP_ThirdPersonCharacter` OtherActor))
  (bind _currenthealth (`/Game/ThirdPerson/Blueprints/BP_ThirdPersonCharacter.CurrentHealth` _asbp_third_person_character))
  (if (> (`/Game/ThirdPerson/Blueprints/BP_ThirdPersonCharacter.MaxHealth` _asbp_third_person_character) _currenthealth)
    (set `/Game/ThirdPerson/Blueprints/BP_ThirdPersonCharacter.CurrentHealth` (+ _currenthealth 1.0) _asbp_third_person_character)
    (`/Game/ThirdPerson/Blueprints/BP_ThirdPersonCharacter.UpdateUI` _asbp_third_person_character)
    (`KismetSystemLibrary.Delay` 0.2)
    (`self.K2_DestroyActor`)
    (`GameplayStatics.PlaySound2D` "/Game/GAME_RELATED/Sounds/HealthRecharge.HealthRecharge" 1.0 1.0 0.0 null null)))

(fn `UserConstructionScript`)