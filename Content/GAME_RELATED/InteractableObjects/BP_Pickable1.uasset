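; BP_Pickable1 is an interactable pickup that tells overlapping actors when they enter or leave its collision box.
; Actors implementing BPI_CharacterAttachmentInteraction receive an overlap status message, with the pickup passing itself as a reference on entry.
; ChangeHoldingStatus records whether the object is held, and exit messages are suppressed while it is.
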(event `self.Box_collision.OnComponentBeginOverlap`
  (params (OverlappedComponent :type "PrimitiveComponent Object Reference") (OtherActor :type "Actor Object Reference") (OtherComp :type "PrimitiveComponent Object Reference") (OtherBodyIndex :type Integer) (bFromSweep :type Boolean) (SweepResult :type "HitResult Structure (by ref)"))
  (if (`KismetSystemLibrary.DoesImplementInterface` OtherActor "/Game/GAME_RELATED/InteractableObjects/BPI_CharacterAttachmentInteraction.BPI_CharacterAttachmentInteraction_C")
    (message `/Game/GAME_RELATED/InteractableObjects/BPI_CharacterAttachmentInteraction.Overlap_StatusChange` OtherActor "NewEnumerator0" self)))

(event `self.Box_collision.OnComponentEndOverlap`
  (params (OverlappedComponent :type "PrimitiveComponent Object Reference") (OtherActor :type "Actor Object Reference") (OtherComp :type "PrimitiveComponent Object Reference") (OtherBodyIndex :type Integer))
  (if (and (`KismetSystemLibrary.DoesImplementInterface` null "/Game/GAME_RELATED/InteractableObjects/BPI_CharacterAttachmentInteraction.BPI_CharacterAttachmentInteraction_C") (not (`self.ObjectPickedUp`)))
    (message `/Game/GAME_RELATED/InteractableObjects/BPI_CharacterAttachmentInteraction.Overlap_StatusChange` OtherActor "NewEnumerator1" null)))

(event `/Game/GAME_RELATED/InteractableObjects/BPI_ObjectAttachment.ChangeHoldingStatus`
  (params (IsHolding :type Boolean))
  (set `self.ObjectPickedUp` IsHolding))

(fn `UserConstructionScript`)