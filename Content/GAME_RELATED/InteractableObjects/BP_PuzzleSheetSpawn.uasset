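; BP_PuzzleSheetSpawn is an activatable object that reveals a puzzle sheet once enough distinct controlling actors have triggered it.
; Unless flagged as spawned from the beginning, it lowers the sheet on BeginPlay and collects unique activators until their count equals the required amount.
; The SheetAppearence timeline then raises the sheet, lerping from its current height toward a fixed relative Z.
; Deactivation does nothing, so activators stay counted.
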(event `self.ReceiveBeginPlay`
  (bind _puzzlesheet (`self.PuzzleSheet`))
  (bind (_relativelocation_x _relativelocation_y _relativelocation_z) (`KismetMathLibrary.BreakVector` (`SceneComponent.RelativeLocation` _puzzlesheet)))
  (if (not (`self.SpawnedFromBeginning`))
    (`SceneComponent.K2_SetRelativeLocation` _puzzlesheet (`KismetMathLibrary.MakeVector` _relativelocation_x _relativelocation_y (- _relativelocation_z 200.0)) false false)))

(event `self.OnActivate`
  (params (ControllingActor :type "Actor Object Reference") (Color :type String))
  (bind _controllingactors (`self.ControllingActors`))
  (bind (_relativelocation_x _relativelocation_y _relativelocation_z) (`KismetMathLibrary.BreakVector` (`SceneComponent.RelativeLocation` (`self.PuzzleSheet`))))
  (if (not (`self.SpawnedFromBeginning`))
    (`KismetArrayLibrary.Array_AddUnique` _controllingactors ControllingActor)
    (if (== (`KismetArrayLibrary.Array_Length` _controllingactors) (`self.RequiredAmount`))
      (bind (_direction _newtrack_0) (`Timeline|SheetAppearence`)
        (:`Update`
          (`SceneComponent.K2_SetRelativeLocation` (`self.PuzzleSheet`) (`KismetMathLibrary.MakeVector` _relativelocation_x _relativelocation_y (`KismetMathLibrary.Lerp` _relativelocation_z 120.0 _newtrack_0)) false false))))))

(event `self.OnDeactivate`
  (params (ControllingActor :type "Actor Object Reference")))

(fn `UserConstructionScript`)