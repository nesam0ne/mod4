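; BP_Collectible is a pickup that the third-person character collects by overlapping it.
; On overlap it increments the character's CollectiblesPicked count and calls UpdateUI.
; It then adds its ID to CollectibleCheck on CustomGameInstance, so the record of collected items outlives the level.
; Finally it destroys itself and plays a 2D pickup sound.
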(event `self.ReceiveActorBeginOverlap`
  (params (OtherActor :type "Actor Object Reference"))
  (bind _asbp_third_person_character (cast `/Game/ThirdPerson/Blueprints/BP_ThirdPersonCharacter` OtherActor))
  (set `/Game/ThirdPerson/Blueprints/BP_ThirdPersonCharacter.CollectiblesPicked` (+ (`/Game/ThirdPerson/Blueprints/BP_ThirdPersonCharacter.CollectiblesPicked` _asbp_third_person_character) 1) _asbp_third_person_character)
  (`/Game/ThirdPerson/Blueprints/BP_ThirdPersonCharacter.UpdateUI` _asbp_third_person_character)
  (bind _ascustom_game_instance (cast `/Game/CustomGameInstance` (`GameplayStatics.GetGameInstance`)))
  (`KismetArrayLibrary.Array_Add` (`/Game/CustomGameInstance.CollectibleCheck` _ascustom_game_instance) (`self.ID`))
  (`self.K2_DestroyActor`)
  (`GameplayStatics.PlaySound2D` "/Game/GAME_RELATED/InteractableObjects/Collectible.Collectible" 1.0 1.0 0.0 null null))

(fn `UserConstructionScript`)