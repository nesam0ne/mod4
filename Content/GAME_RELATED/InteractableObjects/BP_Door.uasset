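; BP_Door is an interactable door that swings open once a required number of unique controlling actors have activated it.
; OnActivate collects controllers and plays a timeline that lerps Door1's current yaw toward -130 degrees, compounding each update rather than using a stored start angle.
; OnDeactivate reverses the timeline from its end without removing any controller.
; BeginPlay sets the timeline's time, not play rate, to the inverse of DoorTime.
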(event `self.ReceiveBeginPlay`
  (`TimelineComponent.SetNewTime` (`self.T_DoorOpening`) (/ 1.0 (`self.DoorTime`))))

(event `self.OnActivate`
  (params (ControllingActor :type "Actor Object Reference") (Color :type String))
  (bind _controllingactors (`self.ControllingActors`))
  (bind (_relativerotation_roll _relativerotation_pitch _relativerotation_yaw) (`KismetMathLibrary.BreakRotator` (`SceneComponent.RelativeRotation` (`self.Door1`))))
  (`KismetArrayLibrary.Array_AddUnique` _controllingactors ControllingActor)
  (if (== (`KismetArrayLibrary.Array_Length` _controllingactors) (`self.RequiredAmount`))
    (bind (_direction _rotationtrack) (`Timeline|T_DoorOpening` :!label _label)
      (:`Update`
        (`SceneComponent.K2_SetRelativeRotation` (`self.Door1`) (`KismetMathLibrary.MakeRotator` 0.0 0.0 (`KismetMathLibrary.Lerp` _relativerotation_yaw -130.0 _rotationtrack)) false false))
      (:`Finished`
        (`KismetSystemLibrary.PrintString` "DoorDone")))))

(event `self.OnDeactivate`
  (params (ControllingActor :type "Actor Object Reference"))
  (goto _label :!via `ReverseFromEnd`))

(fn `UserConstructionScript`)