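; Base NPC that runs dialogue for a note-collection quest and gives per-character hint lines, with Russian text.
; Its collision notifies the player through BPI_dialogues_and_puzzles and animates an interaction hint widget.
; OnInteract switches on NPCType, advancing from intro lines to a sheet count, then at four sheets activating ControlledActor (the elevator, per dialogue).
; W_dialogue displays text while movement is disabled, with FlipFlops toggling non-intro dialogue open and closed.
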(event `self.ReceiveBeginPlay`
  (message `/Game/GAME_RELATED/InteractableObjects/NPC/BPI_Dialogue_UI.OnBegin` (`WidgetComponent.GetWidget` (`self.InteractionHint`)) (`self.NPC_type`))
  (if (and (not (`self.Talked?`)) (`|EnumEquality` (`self.NPC_type`) "NewEnumerator0"))
    (message `/Game/GAME_RELATED/InteractableObjects/NPC/BPI_Dialogue_UI.PlayAnim` (`WidgetComponent.GetWidget` (`self.InteractionHint`)) "NewEnumerator1")))

(event `self.Interaction_collision.OnComponentBeginOverlap`
  (params (OverlappedComponent :type "PrimitiveComponent Object Reference") (OtherActor :type "Actor Object Reference") (OtherComp :type "PrimitiveComponent Object Reference") (OtherBodyIndex :type Integer) (bFromSweep :type Boolean) (SweepResult :type "HitResult Structure (by ref)"))
  (if (and (`KismetSystemLibrary.DoesImplementInterface` OtherActor "/Game/GAME_RELATED/InteractableObjects/NPC/BPI_dialogues_and_puzzles.BPI_dialogues_and_puzzles_C") (== (`GameplayStatics.GetObjectClass` OtherActor) "/Game/ThirdPerson/Blueprints/BP_ThirdPersonCharacter.BP_ThirdPersonCharacter_C"))
    (message `/Game/GAME_RELATED/InteractableObjects/NPC/BPI_dialogues_and_puzzles.Response` OtherActor self)
    (message `/Game/GAME_RELATED/InteractableObjects/NPC/BPI_Dialogue_UI.PlayAnim` (`WidgetComponent.GetWidget` (`self.InteractionHint`)) "NewEnumerator0")))

(event `self.Interaction_collision.OnComponentEndOverlap`
  (params (OverlappedComponent :type "PrimitiveComponent Object Reference") (OtherActor :type "Actor Object Reference") (OtherComp :type "PrimitiveComponent Object Reference") (OtherBodyIndex :type Integer))
  (if (`KismetSystemLibrary.DoesImplementInterface` OtherActor "/Game/GAME_RELATED/InteractableObjects/NPC/BPI_dialogues_and_puzzles.BPI_dialogues_and_puzzles_C")
    (message `/Game/GAME_RELATED/InteractableObjects/NPC/BPI_dialogues_and_puzzles.Response` OtherActor self)
    (`Widget.RemoveFromParent` (`self.UI`))
    (set `self.UI` null)
    (switch `/Game/GAME_RELATED/InteractableObjects/NPC/E_NPC_type` (`self.NPC_type`)
      (:`NewEnumerator0`
        (if (`self.Talked?`)
          (message `/Game/GAME_RELATED/InteractableObjects/NPC/BPI_Dialogue_UI.PlayAnim` (`WidgetComponent.GetWidget` (`self.InteractionHint`)) "NewEnumerator2" :!label _label)
          (else
            (message `/Game/GAME_RELATED/InteractableObjects/NPC/BPI_Dialogue_UI.PlayAnim` (`WidgetComponent.GetWidget` (`self.InteractionHint`)) "NewEnumerator1"))))
      (:`NewEnumerator6`
        (goto _label))
      (:`NewEnumerator7`
        (message `/Game/GAME_RELATED/InteractableObjects/NPC/BPI_Dialogue_UI.PlayAnim` (`WidgetComponent.GetWidget` (`self.InteractionHint`)) "NewEnumerator1"))
      (:`NewEnumerator1`
        (goto _label)))))

(event `/Game/GAME_RELATED/InteractableObjects/NPC/BPI_dialogues_and_puzzles.OnInteract`
  (params (CollectedSheets :type Integer))
  (bind _output_get (set `self.Collected Sheets` CollectedSheets))
  (if (and (== _output_get 4) (`|EnumEquality` (`self.NPC_type`) "NewEnumerator6"))
    (set `self.NPC_type` "NewEnumerator7"))
  (switch `/Game/GAME_RELATED/InteractableObjects/NPC/E_NPC_type` (`self.NPC_type`)
    (:`NewEnumerator0`
      (`/Engine/EditorBlueprintResources/StandardMacros.IncrementInt` (`self.talkindex1`)
        (:`  `
          (if (< (`self.talkindex1`) (`KismetArrayLibrary.Array_Length` (`self.talk_first`)))
            (`/Engine/EditorBlueprintResources/StandardMacros.IsValid` (`self.UI`)
              (:`Is Valid`
                _)
              (:`Is Not Valid`
                (`self.StartDialogueWidget`)))
            (set `TextBlock.Text` (`KismetTextLibrary.Conv_StringToText` (`|GetArrayItem` (`self.talk_first`) (`self.talkindex1`))) (`/Game/GAME_RELATED/InteractableObjects/NPC/W_dialogue.dialogue_text` (`self.UI`)))
            (set `self.Talked?` true)
            (else
              (`Widget.RemoveFromParent` (`self.UI`))
              (set `self.NPC_type` "NewEnumerator6")
              (set `self.UI` null)
              (`CharacterMovementComponent.SetMovementMode` (`Character.CharacterMovement` (`GameplayStatics.GetPlayerCharacter` 0)) "MOVE_Walking" 0)
              (message `/Game/GAME_RELATED/InteractableObjects/NPC/BPI_Dialogue_UI.OnBegin` (`WidgetComponent.GetWidget` (`self.InteractionHint`)) (`self.NPC_type`)))))))
    (:`NewEnumerator6`
      (`/Engine/EditorBlueprintResources/StandardMacros.FlipFlop`
        (:`A`
          (`self.StartDialogueWidget`)
          (set `TextBlock.Text` (`KismetTextLibrary.Conv_StringToText` (`KismetStringLibrary.Concat_StrStr` "Ты принес... " (`KismetStringLibrary.Conv_IntToString` (`self.Collected Sheets`)) ". Возвращайся с 4 записками!")) (`/Game/GAME_RELATED/InteractableObjects/NPC/W_dialogue.dialogue_text` (`self.UI`))))
        (:`B`
          (`/Game/GAME_RELATED/InteractableObjects/NPC/BPI_Dialogue_UI.PlayAnim` (`self.UI`) "NewEnumerator0")
          (set `self.UI` null)
          (`CharacterMovementComponent.SetMovementMode` (`Character.CharacterMovement` (`GameplayStatics.GetPlayerCharacter` 0)) "MOVE_Walking" 0))))
    (:`NewEnumerator7`
      (`/Engine/EditorBlueprintResources/StandardMacros.FlipFlop`
        (:`A`
          (`self.StartDialogueWidget`)
          (set `TextBlock.Text` (`KismetTextLibrary.Conv_StringToText` "Ничего себе! Все 4 записки!  Ну, раз так... Пожалуйста. Лифт открыт!") (`/Game/GAME_RELATED/InteractableObjects/NPC/W_dialogue.dialogue_text` (`self.UI`)))
          (message `/Game/GAME_RELATED/InteractableObjects/BPI_ButtonAction.OnActivate` (`self.ControlledActor`) null ""))
        (:`B`
          (`/Game/GAME_RELATED/InteractableObjects/NPC/BPI_Dialogue_UI.PlayAnim` (`self.UI`) "NewEnumerator0")
          (set `self.UI` null)
          (`CharacterMovementComponent.SetMovementMode` (`Character.CharacterMovement` (`GameplayStatics.GetPlayerCharacter` 0)) "MOVE_Walking" 0))))
    (:`NewEnumerator1`
      (`/Engine/EditorBlueprintResources/StandardMacros.FlipFlop`
        (:`A`
          (`self.StartDialogueWidget`)
          (switch `int` (`self.NPC ID`)
            (:`1`
              (set `self.hint` "Чего ты меня отвлекаешь?! Не видишь что я на середине заполнения документов?! Уйди и не мешай мне!"))
            (:`2`
              (set `self.hint` "Ах, как хорошо быть первой, все делаешь раньше всех и можешь дальше наслаждаться отдыхом."))
            (:`3`
              (set `self.hint` "Ох… Как мне нравится тот, что злой. Всегда стою за ним, когда есть возможность."))
            (:`4`
              (set `self.hint` "Вся эта суета так выматывает. Благо мне удается выполнить все задания, но только под конец дня."))
            (:`5`
              (set `self.hint` "Ну почему! Почему я всегда нахожусь между зазнайкой и ненормальным. Вечно приходится выслушивать самовлюбленные речи и недовольство.")))
          (set `TextBlock.Text` (`KismetTextLibrary.Conv_StringToText` (`self.hint`)) (`/Game/GAME_RELATED/InteractableObjects/NPC/W_dialogue.dialogue_text` (`self.UI`))))
        (:`B`
          (`/Game/GAME_RELATED/InteractableObjects/NPC/BPI_Dialogue_UI.PlayAnim` (`self.UI`) "NewEnumerator0")
          (set `self.UI` null)
          (`CharacterMovementComponent.SetMovementMode` (`Character.CharacterMovement` (`GameplayStatics.GetPlayerCharacter` 0)) "MOVE_Walking" 0))))))

(fn `StartDialogueWidget`
  (`CharacterMovementComponent.SetMovementMode` (`Character.CharacterMovement` (`GameplayStatics.GetPlayerCharacter` 0)) "MOVE_None" 0)
  (bind _returnvalue (`|CreateWidget` "/Game/GAME_RELATED/InteractableObjects/NPC/W_dialogue.W_dialogue_C" (`GameplayStatics.GetPlayerController` 0)))
  (bind _output_get (set `self.UI` _returnvalue))
  (message `/Game/GAME_RELATED/InteractableObjects/NPC/BPI_Dialogue_UI.PlayAnim` _output_get "NewEnumerator2")
  (`UserWidget.AddToViewport` _output_get 0))

(fn `UserConstructionScript`)