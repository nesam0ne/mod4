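; BP_PickableCube is an interactable cube that characters can pick up.
; Its collision box reports overlap begin and end to actors implementing BPI_CharacterAttachmentInteraction, passing itself on begin and suppressing the end message while ObjectPickedUp is set.
; The construction script applies the Material variable to the mesh, and the ChangeHoldingStatus event is an empty stub.
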(event `self.Box_collision.OnComponentBeginOverlap`
  (params (OverlappedComponent :type "PrimitiveComponent Object Reference") (OtherActor :type "Actor Object Reference") (OtherComp :type "PrimitiveComponent Object Reference") (OtherBodyIndex :type Integer) (bFromSweep :type Boolean) (SweepResult :type "HitResult Structure (by ref)"))
  (if (`KismetSystemLibrary.DoesImplementInterface` OtherActor "/Game/GAME_RELATED/InteractableObjects/PickingObjectsCode/BPI_CharacterAttachmentInteraction.BPI_CharacterAttachmentInteraction_C")
    (message `/Game/GAME_RELATED/InteractableObjects/PickingObjectsCode/BPI_CharacterAttachmentInteraction.Overlap_StatusChange` OtherActor "NewEnumerator0" self)))

(event `self.Box_collision.OnComponentEndOverlap`
  (params (OverlappedComponent :type "PrimitiveComponent Object Reference") (OtherActor :type "Actor Object Reference") (OtherComp :type "PrimitiveComponent Object Reference") (OtherBodyIndex :type Integer))
  (if (and (`KismetSystemLibrary.DoesImplementInterface` null "/Game/GAME_RELATED/InteractableObjects/PickingObjectsCode/BPI_CharacterAttachmentInteraction.BPI_CharacterAttachmentInteraction_C") (not (`self.ObjectPickedUp`)))
    (message `/Game/GAME_RELATED/InteractableObjects/PickingObjectsCode/BPI_CharacterAttachmentInteraction.Overlap_StatusChange` OtherActor "NewEnumerator1" null)))

(event `/Game/GAME_RELATED/InteractableObjects/PickingObjectsCode/BPI_ObjectAttachment.ChangeHoldingStatus`
  (params (IsHolding :type Boolean)))

(fn `UserConstructionScript`
  (`PrimitiveComponent.SetMaterial` (`self.Mesh`) 0 (`self.Material`)))