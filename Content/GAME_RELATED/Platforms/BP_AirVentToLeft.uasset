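; Air vent platform that catches a gliding BP_ThirdPersonCharacter and lifts it while pausing stamina drain.
; TeleportBox pulls the glider to FloatingBox with a swept Timeline lerp that stops if gliding ends, rechecking non-gliders on a delay loop.
; FloatingBox launches gliders upward and replenishes stamina.
; Leaving FloatCheck or TeleportBox while gliding restores stamina drain after a delay.
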(event `self.FloatingBox.OnComponentBeginOverlap`
  (params (OverlappedComponent :type "PrimitiveComponent Object Reference") (OtherActor :type "Actor Object Reference") (OtherComp :type "PrimitiveComponent Object Reference") (OtherBodyIndex :type Integer) (bFromSweep :type Boolean) (SweepResult :type "HitResult Structure (by ref)"))
  (bind _asbp_third_person_character (cast `/Game/ThirdPerson/Blueprints/BP_ThirdPersonCharacter` OtherActor))
  (if (`/Game/ThirdPerson/Blueprints/BP_ThirdPersonCharacter.IsGliding` _asbp_third_person_character)
    (set `/Game/ThirdPerson/Blueprints/BP_ThirdPersonCharacter.IsWastingStamina` false _asbp_third_person_character)
    (`Character.LaunchCharacter` _asbp_third_person_character (0.0 0.0 200.0) false true)
    (`/Game/ThirdPerson/Blueprints/BP_ThirdPersonCharacter.Replenish Stamina` _asbp_third_person_character)))

(event `self.FloatCheck.OnComponentEndOverlap`
  (params (OverlappedComponent :type "PrimitiveComponent Object Reference") (OtherActor :type "Actor Object Reference") (OtherComp :type "PrimitiveComponent Object Reference") (OtherBodyIndex :type Integer))
  (`KismetSystemLibrary.RetriggerableDelay` 1.0)
  (bind _asbp_third_person_character (cast `/Game/ThirdPerson/Blueprints/BP_ThirdPersonCharacter` OtherActor))
  (if (`/Game/ThirdPerson/Blueprints/BP_ThirdPersonCharacter.IsGliding` _asbp_third_person_character)
    (set `/Game/ThirdPerson/Blueprints/BP_ThirdPersonCharacter.IsWastingStamina` true _asbp_third_person_character)
    (`/Game/ThirdPerson/Blueprints/BP_ThirdPersonCharacter.Consume Stamina` _asbp_third_person_character 0.2)))

(event `self.TeleportBox.OnComponentBeginOverlap`
  (params (OverlappedComponent :type "PrimitiveComponent Object Reference") (OtherActor :type "Actor Object Reference") (OtherComp :type "PrimitiveComponent Object Reference") (OtherBodyIndex :type Integer) (bFromSweep :type Boolean) (SweepResult :type "HitResult Structure (by ref)"))
  (bind (_returnvalue_x _returnvalue_y _returnvalue_z) (`KismetMathLibrary.BreakVector` (`SceneComponent.K2_GetComponentLocation` (`self.FloatingBox`))))
  (bind _asbp_third_person_character (cast `/Game/ThirdPerson/Blueprints/BP_ThirdPersonCharacter` OtherActor))
  (bind _isgliding (`/Game/ThirdPerson/Blueprints/BP_ThirdPersonCharacter.IsGliding` _asbp_third_person_character))
  (if _isgliding :!label _label
    (set `/Game/ThirdPerson/Blueprints/BP_ThirdPersonCharacter.IsWastingStamina` false _asbp_third_person_character)
    (bind _output_get (set `self.StartLoc` (`self.K2_GetActorLocation` _asbp_third_person_character)))
    (bind _outhit (`KismetSystemLibrary.LineTraceSingle` :`Start` _output_get :`End` (`KismetMathLibrary.MakeVector` _returnvalue_x _returnvalue_y _returnvalue_z) :`TraceChannel` "TraceTypeQuery1" :`DrawDebugType` "ForDuration" :`DrawTime` 20.0))
    (bind (_direction _newtrack_0) (`Timeline|Timeline_0` :!via `PlayFromStart` :!label _label_2)
      (:`Update`
        (if _isgliding
          (`self.K2_SetActorLocation` _asbp_third_person_character (`KismetMathLibrary.VLerp` (`self.StartLoc`) (`.TraceEnd` (`GameplayStatics.BreakHitResult` _outhit)) _newtrack_0) true false)
          (else
            (goto _label_2 :!via `Stop`)))))
    (else
      (`KismetSystemLibrary.Delay` 0.3)
      (`/Engine/EditorBlueprintResources/StandardMacros.IsValid` OtherActor
        (:`Is Valid`
          (goto _label))))))

(event `self.TeleportBox.OnComponentEndOverlap`
  (params (OverlappedComponent :type "PrimitiveComponent Object Reference") (OtherActor :type "Actor Object Reference") (OtherComp :type "PrimitiveComponent Object Reference") (OtherBodyIndex :type Integer))
  (bind _asbp_third_person_character (cast `/Game/ThirdPerson/Blueprints/BP_ThirdPersonCharacter` OtherActor))
  (if (`/Game/ThirdPerson/Blueprints/BP_ThirdPersonCharacter.IsGliding` _asbp_third_person_character)
    (`KismetSystemLibrary.Delay` 2.0)
    (set `/Game/ThirdPerson/Blueprints/BP_ThirdPersonCharacter.IsWastingStamina` true _asbp_third_person_character)
    (else
      (set `/Game/ThirdPerson/Blueprints/BP_ThirdPersonCharacter.IsWastingStamina` false _asbp_third_person_character))))

(fn `Floating`)

(fn `UserConstructionScript`)