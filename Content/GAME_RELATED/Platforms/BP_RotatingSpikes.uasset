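; BP_RotatingSpikes is a spike platform actor that flips 180 degrees around its roll axis each time its Rotate event is called.
; An IsFinished flag ignores calls made mid-flip, and each flip starts from the root component's current world rotation.
; A MultiGate alternates between two timelines, resetting after the second, with both lerping roll in the same direction and setting actor rotation with physics teleport.
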(event `Rotate`
  (bind (_currentrotation_roll _currentrotation_pitch _currentrotation_yaw) (`KismetMathLibrary.BreakRotator` (`self.CurrentRotation`)))
  (bind _currentrotation_roll_2 (`KismetMathLibrary.BreakRotator` (`self.CurrentRotation`)))
  (bind _currentrotation_roll_3 (`KismetMathLibrary.BreakRotator` (`self.CurrentRotation`)))
  (bind (_currentrotation_roll_4 _currentrotation_pitch_2 _currentrotation_yaw_2) (`KismetMathLibrary.BreakRotator` (`self.CurrentRotation`)))
  (if (`self.IsFinished`)
    (set `self.CurrentRotation` (`SceneComponent.K2_GetComponentRotation` (`self.DefaultSceneRoot`)))
    (`|MultiGate` false :!label _label
      (:`Out 0`
        (set `self.IsFinished` false)
        (bind (_direction _newtrack_0) (`Timeline|RotationTimeline` :!via `PlayFromStart`)
          (:`Update`
            (`self.K2_SetActorRotation` (`KismetMathLibrary.MakeRotator` (`KismetMathLibrary.Lerp` _currentrotation_roll_2 (- _currentrotation_roll_2 180.0) _newtrack_0) _currentrotation_pitch _currentrotation_yaw) true))
          (:`Finished`
            (set `self.IsFinished` true))))
      (:`Out 1`
        (set `self.IsFinished` false)
        (bind (_direction_2 _newtrack_0_2) (`Timeline|Timeline` :!via `PlayFromStart`)
          (:`Update`
            (`self.K2_SetActorRotation` (`KismetMathLibrary.MakeRotator` (`KismetMathLibrary.Lerp` _currentrotation_roll_3 (- _currentrotation_roll_3 180.0) _newtrack_0_2) _currentrotation_pitch_2 _currentrotation_yaw_2) true))
          (:`Finished`
            (set `self.IsFinished` true)
            (goto _label :!via `Reset`)))))))

(fn `UserConstructionScript`)