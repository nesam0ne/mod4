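; BP_AirVentLevel is an air vent platform that lifts a gliding BP_ThirdPersonCharacter while it is inside the Box volume.
; Entering gives a strong upward launch and pauses stamina waste, then starts the Floating event.
; Floating calls itself through a retriggerable delay, repeating a weaker Z-override launch while gliding continues.
; Leaving stops the loop and resumes stamina waste if still gliding.
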(event `self.Box.OnComponentBeginOverlap`
  (params (OverlappedComponent :type "PrimitiveComponent Object Reference") (OtherActor :type "Actor Object Reference") (OtherComp :type "PrimitiveComponent Object Reference") (OtherBodyIndex :type Integer) (bFromSweep :type Boolean) (SweepResult :type "HitResult Structure (by ref)"))
  (bind _asbp_third_person_character (cast `/Game/ThirdPerson/Blueprints/BP_ThirdPersonCharacter` OtherActor))
  (if (`/Game/ThirdPerson/Blueprints/BP_ThirdPersonCharacter.IsGliding` _asbp_third_person_character)
    (set `/Game/ThirdPerson/Blueprints/BP_ThirdPersonCharacter.IsWastingStamina` false _asbp_third_person_character)
    (`Character.LaunchCharacter` _asbp_third_person_character (0.0 0.0 400.0) false true)
    (set `self.floatingStop` false)
    (`self.Floating`)))

(event `Floating`
  (if (and (not (`self.floatingStop`)) (`/Game/ThirdPerson/Blueprints/BP_ThirdPersonCharacter.IsGliding` (stale `self.Box.OnComponentBeginOverlap` _asbp_third_person_character)))
    (`KismetSystemLibrary.RetriggerableDelay` 0.3)
    (`Character.LaunchCharacter` (stale `self.Box.OnComponentBeginOverlap` _asbp_third_person_character) (0.0 0.0 150.0) false true)
    (`self.Floating`)
    (set `/Game/ThirdPerson/Blueprints/BP_ThirdPersonCharacter.IsWastingStamina` false (stale `self.Box.OnComponentBeginOverlap` _asbp_third_person_character))))

(event `self.Box.OnComponentEndOverlap`
  (params (OverlappedComponent :type "PrimitiveComponent Object Reference") (OtherActor :type "Actor Object Reference") (OtherComp :type "PrimitiveComponent Object Reference") (OtherBodyIndex :type Integer))
  (set `self.floatingStop` true)
  (bind _asbp_third_person_character (cast `/Game/ThirdPerson/Blueprints/BP_ThirdPersonCharacter` (stale `self.Box.OnComponentBeginOverlap` OtherActor)))
  (if (`/Game/ThirdPerson/Blueprints/BP_ThirdPersonCharacter.IsGliding` _asbp_third_person_character)
    (set `/Game/ThirdPerson/Blueprints/BP_ThirdPersonCharacter.IsWastingStamina` true _asbp_third_person_character)))

(fn `UserConstructionScript`)