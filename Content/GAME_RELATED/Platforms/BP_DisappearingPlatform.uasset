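; BP_DisappearingPlatform is a platform that fades out and stops being solid after the third-person character touches it, then returns after a delay.
; An overlap on PlayerCheck plays the DisSequence timeline, which drives Opacity on a dynamic material instance.
; When it finishes, both components ignore collision until RespawnTimeline starts restoring opacity and collision after RespawnTime.
; BeginPlay passes the inverse of SecondsUntilDisappears to SetNewTime, which sets timeline position rather than play rate.
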(event `self.ReceiveBeginPlay`
  (bind _returnvalue (`PrimitiveComponent.CreateDynamicMaterialInstance` (`self.DisappearingPlatform`) 0 "/Game/GAME_RELATED/Platforms/M_DisappearingPlatform.M_DisappearingPlatform" "None"))
  (bind _output_get (set `self.LocalMaterial` _returnvalue))
  (`MaterialInstanceDynamic.SetScalarParameterValue` (`self.LocalMaterial`) "Bright" 0.0)
  (`MaterialInstanceDynamic.SetScalarParameterValue` _output_get "Bright" 0.0)
  (`TimelineComponent.SetNewTime` (`self.DisSequence`) (/ 1.0 (`self.Seconds Until Disappears`)))
  (`TimelineComponent.SetNewTime` (`self.RespawnTimeline`) (/ 1.0 (`self.Seconds Until Disappears`))))

(event `self.PlayerCheck.OnComponentBeginOverlap`
  (params (OverlappedComponent :type "PrimitiveComponent Object Reference") (OtherActor :type "Actor Object Reference") (OtherComp :type "PrimitiveComponent Object Reference") (OtherBodyIndex :type Integer) (bFromSweep :type Boolean) (SweepResult :type "HitResult Structure (by ref)"))
  (if (== (`GameplayStatics.GetObjectClass` OtherActor) "/Game/ThirdPerson/Blueprints/BP_ThirdPersonCharacter.BP_ThirdPersonCharacter_C")
    (bind (_direction _newtrack_0) (`Timeline|DisSequence` :!via `PlayFromStart`)
      (:`Update`
        (`MaterialInstanceDynamic.SetScalarParameterValue` (`self.LocalMaterial`) "Opacity" _newtrack_0))
      (:`Finished`
        (`PrimitiveComponent.SetCollisionResponseToAllChannels` (`self.DisappearingPlatform`) "ECR_Ignore")
        (`PrimitiveComponent.SetCollisionResponseToAllChannels` (`self.PlayerCheck`) "ECR_Ignore")
        (`KismetSystemLibrary.Delay` (`self.RespawnTime`))
        (bind (_direction_2 _newtrack_0_2) (`Timeline|RespawnTimeline` :!via `PlayFromStart`)
          (:`Update`
            (`MaterialInstanceDynamic.SetScalarParameterValue` (`self.LocalMaterial`) "Opacity" _newtrack_0_2)
            (`PrimitiveComponent.SetCollisionResponseToAllChannels` (`self.DisappearingPlatform`) "ECR_Block")
            (`PrimitiveComponent.SetCollisionResponseToAllChannels` (`self.PlayerCheck`) "ECR_Overlap")))))))

(fn `UserConstructionScript`)