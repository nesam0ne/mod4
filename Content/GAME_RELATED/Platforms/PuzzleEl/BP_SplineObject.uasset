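; Puzzle platform object that, on activation, travels along a referenced spline actor.
; A timeline maps its track to distance along the spline, setting the actor's world location and rotation.
; When the timeline finishes at the spline's end, it sends an activate message to its controlled actor.
; Overlapping AirVentCheck with an upward air vent pickable reverses the movement.
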(event `self.ReceiveBeginPlay`
  (`TimelineComponent.SetNewTime` (`self.T_Move`) (/ 1.0 (`self.TimeToComplete`))))

(event `/Game/GAME_RELATED/InteractableObjects/BPI_ButtonAction.OnActivate`
  (params (ControllingActor :type "Actor Object Reference") (Color :type String))
  (bind _spline (`/Game/GAME_RELATED/Platforms/PuzzleEl/BP_SplinePath.Spline` (`self.SplineToFollow`)))
  (`/Engine/EditorBlueprintResources/StandardMacros.IsValid` (`self.SplineToFollow`)
    (:`Is Valid`
      (bind (_direction _movetrack) (`Timeline|T_Move` :!via `PlayFromStart` :!label _label)
        (:`Update`
          (bind _returnvalue (`KismetMathLibrary.Lerp` 0.0 (`SplineComponent.GetSplineLength` _spline) _movetrack))
          (`self.K2_SetActorLocationAndRotation` (`SplineComponent.GetLocationAtDistanceAlongSpline` _spline _returnvalue "World") (`SplineComponent.GetRotationAtDistanceAlongSpline` _spline _returnvalue "World")))
        (:`Finished`
          (if (== _movetrack 1.0)
            (message `/Game/GAME_RELATED/InteractableObjects/BPI_ButtonAction.OnActivate` (`self.ControlledActor`) self "")))))
    (:`Is Not Valid`
      (`KismetSystemLibrary.PrintString` "NotValid"))))

(event `self.AirVentCheck.OnComponentBeginOverlap`
  (params (OverlappedComponent :type "PrimitiveComponent Object Reference") (OtherActor :type "Actor Object Reference") (OtherComp :type "PrimitiveComponent Object Reference") (OtherBodyIndex :type Integer) (bFromSweep :type Boolean) (SweepResult :type "HitResult Structure (by ref)"))
  (if (== (`GameplayStatics.GetObjectClass` OtherActor) "/Game/GAME_RELATED/Platforms/BP_AirVentUp_Pickable.BP_AirVentUp_Pickable_C")
    (goto _label :!via `Reverse`)))

(fn `UserConstructionScript`)